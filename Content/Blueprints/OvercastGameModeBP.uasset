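; Game mode for Overcast that handles pausing and saving progress to a save slot.
; ToggleGamePaused flips the pause state, shows the mouse cursor while paused and tells GameHUDBP to update.
; SaveGame writes the current level index, checkpoint index and Player1's unlocked spells into an OvercastSaveGameBP, then prints success or failure.
; GetMenuLevelName returns only None, and Tick is empty.
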(event EventTick
  (params (DeltaSeconds :type Float%20%28single-precision%29)))

(fn ConstructionScript)

(fn GetMenuLevelName
  (return "None"))

(fn ToggleGamePaused
  (bind _returnvalue (Game|GetPlayerController 0))
  (bind _returnvalue_2 (Game|IsGamePaused))
  (Game|SetGamePaused (not _returnvalue_2))
  (Variables|/Script/Engine.PlayerController|SetbShowMouseCursor _returnvalue _returnvalue_2)
  (bind _asgame_hudbp (Utilities|Casting|CastToGameHUDBP (HUD|GetHUD _returnvalue)))
  (Default|UpdatePaused _asgame_hudbp))

(fn SaveGame
  (bind _returnvalue (SaveGame|CreateSaveGameObject "/Game/Blueprints/OvercastSaveGameBP.OvercastSaveGameBP_C"))
  (Variables|/Game/Blueprints/OvercastSaveGameBP.OvercastSaveGameBP_C|SetLevelIndex _returnvalue (Variables|Default|GetCurrentLevelIndex))
  (Variables|/Game/Blueprints/OvercastSaveGameBP.OvercastSaveGameBP_C|SetCheckpointIndex _returnvalue (Variables|Default|GetCurrentCheckpointIndex))
  (bind _asplayer_1 (Utilities|Casting|CastToPlayer1 (Game|GetPlayerCharacter 0)))
  (Variables|/Game/Blueprints/OvercastSaveGameBP.OvercastSaveGameBP_C|SetUnlockedSpells _returnvalue (Class|Player1|GetUnlockedSpells _asplayer_1))
  (bind _returnvalue_2 (SaveGame|SaveGametoSlot _returnvalue "overcastSave"))
  (if _returnvalue_2
    (Development|PrintString "SvaeGmaeCplmelte")
    (else
      (Development|PrintString "big Fail on save"))))