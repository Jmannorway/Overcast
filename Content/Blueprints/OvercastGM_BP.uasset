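; Overcast game manager, apparently the game mode, that handles player respawning, pausing and the menu level name.
; It binds to the player pawn's OnDestroyed at BeginPlay, then after a short delay spawns a new Player1_BP at SpawnTransform, possesses it and rebinds.
; ToggleGamePaused flips pause, matches mouse cursor visibility to it and tells GameHUDBP to update.
; GetMenuLevelName exposes the stored menu level name.
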(event Custom|OnDestroyed_Event_0
  (params (DestroyedActor :type Actor%20Object%20Reference))
  (Utilities|FlowControl|Delay 1.0)
  (bind _returnvalue (Game|SpawnActorfromClass "/Game/Blueprints/Player1_BP.Player1_BP_C" (Variables|Default|GetSpawn%20Transform) "Undefined" 0 0))
  (Pawn|Possess (Game|GetPlayerController 0) _returnvalue)
  (CallFunction|Respawn))

(event Custom|Respawn
  (bind _asplayer_1_bp (Utilities|Casting|CastToPlayer1_BP (Game|GetPlayerCharacter 0)))
  (Game|BindEventtoOnDestroyed _asplayer_1_bp (delegate Custom|OnDestroyed_Event_0)))

(event EventBeginPlay
  (bind _asplayer_1_bp (Utilities|Casting|CastToPlayer1_BP (Game|GetPlayerCharacter 0)))
  (Game|BindEventtoOnDestroyed _asplayer_1_bp (delegate Custom|OnDestroyed_Event_0)))

(event EventTick
  (params (DeltaSeconds :type Float%20%28single-precision%29)))

(fn ConstructionScript)

(fn GetMenuLevelName
  (return (Variables|Default|GetMenuLevelName)))

(fn ToggleGamePaused
  (bind _returnvalue (Game|GetPlayerController 0))
  (bind _returnvalue_2 (Game|IsGamePaused))
  (Game|SetGamePaused (not _returnvalue_2))
  (Variables|/Script/Engine.PlayerController|SetbShowMouseCursor _returnvalue _returnvalue_2)
  (bind _asgame_hudbp (Utilities|Casting|CastToGameHUDBP (HUD|GetHUD _returnvalue)))
  (Default|UpdatePaused _asgame_hudbp))