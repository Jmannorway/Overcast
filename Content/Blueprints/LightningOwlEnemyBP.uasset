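; Lightning owl enemy that targets the player, turns to face them and attacks with a lightning projectile.
; Vision overlap sets or clears the target, and Tick updates the owl's yaw toward it.
; Entering Threshhold spawns a projectile linked to owl and target; leaving the separate Range volume destroys it.
; Player death also destroys a live projectile and clears the target, but leaves IsAttacking set.
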(event OnComponentBeginOverlap(Threshhold)
  (params (OverlappedComponent :type Primitive%20Component%20Object%20Reference) (OtherActor :type Actor%20Object%20Reference) (OtherComp :type Primitive%20Component%20Object%20Reference) (OtherBodyIndex :type Integer) (bFromSweep :type Boolean) (SweepResult :type Hit%20Result%20Structure%20%28by%20ref%29))
  (if (== (Variables|Default|GetTargetActor) OtherActor)
    (bind _returnvalue (Game|SpawnActorfromClass "/Game/Blueprints/LightningOwlProjectileBP.LightningOwlProjectileBP_C" (Math|Transform|MakeTransform (Transformation|GetActorLocation) "0, 0, 0" "1,1,1") "Undefined" 0 0))
    (bind _output_get (Variables|Default|SetLightningProjectile _returnvalue))
    (Default|SetTargetActor _output_get (Variables|Default|GetTargetActor))
    (Default|SetSourceActor _output_get self)
    (Variables|Default|SetIsAttacking true)))

(event OnComponentEndOverlap(Range)
  (params (OverlappedComponent :type Primitive%20Component%20Object%20Reference) (OtherActor :type Actor%20Object%20Reference) (OtherComp :type Primitive%20Component%20Object%20Reference) (OtherBodyIndex :type Integer))
  (if (and (== (Variables|Default|GetTargetActor) OtherActor) (Utilities|IsValid (Variables|Default|GetLightningProjectile)))
    (Actor|DestroyActor (Variables|Default|GetLightningProjectile))
    (Variables|Default|SetLightningProjectile 0)
    (Variables|Default|SetIsAttacking false)))

(event OnComponentBeginOverlap(Vision)
  (params (OverlappedComponent :type Primitive%20Component%20Object%20Reference) (OtherActor :type Actor%20Object%20Reference) (OtherComp :type Primitive%20Component%20Object%20Reference) (OtherBodyIndex :type Integer) (bFromSweep :type Boolean) (SweepResult :type Hit%20Result%20Structure%20%28by%20ref%29))
  (bind _asplayer_1_bp (Utilities|Casting|CastToPlayer1_BP OtherActor))
  (Variables|Default|SetTargetActor _asplayer_1_bp))

(event OnComponentEndOverlap(Vision)
  (params (OverlappedComponent :type Primitive%20Component%20Object%20Reference) (OtherActor :type Actor%20Object%20Reference) (OtherComp :type Primitive%20Component%20Object%20Reference) (OtherBodyIndex :type Integer))
  (if (== (Variables|Default|GetTargetActor) OtherActor)
    (Variables|Default|SetTargetActor 0)))

(event EventBeginPlay)

(event Collision|EventActorBeginOverlap
  (params (OtherActor :type Actor%20Object%20Reference)))

(event EventTick
  (params (DeltaSeconds :type Float%20%28single-precision%29))
  (bind _lightningprojectile (Variables|Default|GetLightningProjectile))
  (if (Utilities|IsValid (Variables|Default|GetTargetActor))
    (bind _asplayer_1_bp (Utilities|Casting|CastToPlayer1_BP (Variables|Default|GetTargetActor)))
    (if (Utilities|Enum|Equal(Enum) (Variables|/Script/Overcast.Player1|GetPlayerMovementState _asplayer_1_bp) "Dead")
      (if (Utilities|IsValid _lightningprojectile)
        (Actor|DestroyActor _lightningprojectile)
        (Variables|Default|SetTargetActor 0))
      (else
        (CallFunction|LookatTarget)))))

(fn ConstructionScript)

(fn LookatTarget
  (Transformation|SetActorRotation (Math|Rotator|MakeRotator 0.0 0.0 (+ (.yaw (Math|Rotator|FindLookatRotation (Transformation|GetActorLocation (Variables|Default|GetTargetActor)) (Transformation|GetActorLocation))) 9e+01))))

(fn GetIsAttacking
  (return (Variables|Default|GetIsAttacking)))