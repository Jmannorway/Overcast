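; Lightning owl projectile actor that travels toward an assigned target and sets any Player1 overlapping its sphere to the Dead movement state.
; Each tick, while source and target are valid, it steps at ProjectileSpeed without sweeping, snapping onto the target once within one step.
; The step applies a world-space direction as a local offset.
; Particle actor parameters link the source actor to the projectile itself as the effect's target.
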(event OnComponentBeginOverlap(Sphere)
  (params (OverlappedComponent :type Primitive%20Component%20Object%20Reference) (OtherActor :type Actor%20Object%20Reference) (OtherComp :type Primitive%20Component%20Object%20Reference) (OtherBodyIndex :type Integer) (bFromSweep :type Boolean) (SweepResult :type Hit%20Result%20Structure%20%28by%20ref%29))
  (bind _asplayer_1 (Utilities|Casting|CastToPlayer1 OtherActor))
  (Class|Player1|SetPlayerMovementState _asplayer_1 "Dead"))

(event EventBeginPlay
  (Effects|Components|ParticleSystem|SetActorParameter (Variables|Default|GetParticleSystem) "Target" self))

(event EventTick
  (params (DeltaSeconds :type Float%20%28single-precision%29))
  (if (and (Utilities|IsValid (Variables|Default|GetTargetActor)) (Utilities|IsValid (Variables|Default|GetSourceActor)))
    (CallFunction|MoveTowardsTargetActor DeltaSeconds)))

(fn ConstructionScript)

(fn SetTargetActor
  (params (NewTargetActor :type Actor%20Object%20Reference))
  (Variables|Default|SetTargetActor NewTargetActor))

(fn SetSourceActor
  (params (NewSourceActor :type Actor%20Object%20Reference))
  (bind _output_get (Variables|Default|SetSourceActor NewSourceActor))
  (Effects|Components|ParticleSystem|SetActorParameter (Variables|Default|GetParticleSystem) "Source" _output_get))

(fn MoveTowardsTargetActor
  (params (DeltaTime :type Float%20%28single-precision%29))
  (bind _returnvalue (Transformation|GetActorLocation))
  (bind _targetactor (Variables|Default|GetTargetActor))
  (bind _returnvalue_2 (Transformation|GetActorLocation _targetactor))
  (LocalVariables|SetProjectileTickSpeed (* (Variables|Default|GetProjectileSpeed) DeltaTime))
  (if (> (Math|Vector|Distance(Vector) _returnvalue_2 _returnvalue) (LocalVariables|GetProjectileTickSpeed))
    (Transformation|AddActorLocalOffset (* (Math|Vector|Normalize (- _returnvalue_2 _returnvalue)) (LocalVariables|GetProjectileTickSpeed)) false false)
    (else
      (Transformation|SetActorLocation (Transformation|GetActorLocation (Variables|Default|GetTargetActor)) false false))))